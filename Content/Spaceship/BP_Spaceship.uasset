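; Player spaceship pawn for an asteroid-shooting game, with an HUD asteroid countdown that leads to a victory screen at zero.
; Enhanced Input drives force-based thrust, steering, boost and rate-limited laser components, with speed clamped each tick.
; Tick also updates camera FOV and shake, cosmetic tilt, thruster and particle effects.
; Change detection and filtered hits fire events that feed FMOD parameters for thrusters, steering, collisions and adaptive music.
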(event `self.ReceiveBeginPlay`
  ;[0.03 0.03 0.03] Event Begin Play
  (`self.SetupInputMappingContext`)
  (`self.StartCameraShakeNoise`)
  (`self.AssignLaserProjectileComponents`)
  (`self.SetupMaterials`)
  (`self.StartInitialCameraFade`)
  (bind _returnvalue (`|CreateWidget` "/Game/HUD_Widget.HUD_Widget_C"))
  (bind _output_get (set `self.HUD_Widget` _returnvalue))
  (`UserWidget.AddToViewport` _output_get 0)
  (set `self.Counter` 10)
  (`TextBlock.SetText` (`/Game/HUD_Widget.NumAsteroids` (`self.HUD_Widget`)) (`KismetTextLibrary.Conv_IntToText` (`self.Counter`)))
  ; Crear Instancia Ambience
  (bind _returnvalue_2 (`FMODBlueprintStatics.PlayEvent2D` "/Game/FMOD/Events/Ambience/Ambience.Ambience"))
  (set `self.Ambience` _returnvalue_2)
  ; Crear instancia de evento steering
  (bind _returnvalue_3 (`FMODBlueprintStatics.PlayEvent2D` "/Game/FMOD/Events/Spaceship/Steering.Steering"))
  (set `self.Steering` _returnvalue_3)
  ; Crear componentes para thrusts
  (bind _returnvalue_4 (`FMODBlueprintStatics.PlayEventAttached` "/Game/FMOD/Events/Spaceship/Thrusters_Easy.Thrusters_Easy" (`self.SM_ThrusterInner_Left`) "None" (0.0 0.0 0.0) "KeepRelativeOffset"))
  (set `self.ThrustEvent_L` _returnvalue_4)
  (bind _returnvalue_5 (`FMODBlueprintStatics.PlayEventAttached` "/Game/FMOD/Events/Spaceship/Thrusters_Easy.Thrusters_Easy" (`self.SM_ThrusterInner_Right`) "None" (0.0 0.0 0.0) "KeepRelativeOffset"))
  (set `self.ThrustEvent_R` _returnvalue_5)
  ; Crear instancia de Music
  (bind _returnvalue_6 (`FMODBlueprintStatics.PlayEvent2D` "/Game/FMOD/Events/Music/MainTheme.MainTheme"))
  (bind _output_get_2 (set `self.Music` _returnvalue_6))
  (`FMODBlueprintStatics.EventInstanceSetParameter` _output_get_2 "Game"))

(event `self.ReceiveTick`
  (params (DeltaSeconds :type "Float (single-precision)"))
  ;[0.03 0.03 0.03] Event Tick
  (`self.UpdateMovement`)
  (`self.CheckForBoosting`)
  (`self.UpdateShootingLasers`)
  (`self.UpdateCosmetics`)
  (`self.UpdateCamera`)
  (set `self.wasBoostingLastFrame` (`self.GetIsBoosting`)))

(event `EnhancedInput|/Game/Input/IA_Steer`
  (params (ActionValue :type "Vector2D Structure") (ElapsedSeconds :type "Float (double-precision)") (TriggeredSeconds :type "Float (double-precision)") (InputAction :type "InputAction Object Reference" :default "/Game/Input/IA_Steer.IA_Steer"))
  ;[0.03 0.03 0.03] Input
  (:`Triggered`
    (set `self.steerInputX` ActionValue_X :!label _label)
    (set `self.steerInputY` (`KismetMathLibrary.SelectFloat` (* ActionValue_Y -1.0) ActionValue_Y (`self.ShouldInvertYMovement`)))
    (`|ExecutionSequence`
      (:`then_0`
        (if (or (!= (`self.steerInputX`) (`self.steerInputXLastFrame`)) (!= (`self.steerInputY`) (`self.steerInputYLastFrame`)))
          (`self.OnSteerInputChanged` (`self.steerInputX`) (`self.steerInputY`))))
      (:`then_1`
        (set `self.steerInputXLastFrame` (`self.steerInputX`))
        (set `self.steerInputYLastFrame` (`self.steerInputY`)))))
  (:`Started`
    (goto _label))
  (:`Completed`
    (goto _label)))

(event `EnhancedInput|/Game/Input/IA_Thrust`
  (params (ActionValue :type "Float (double-precision)") (ElapsedSeconds :type "Float (double-precision)") (TriggeredSeconds :type "Float (double-precision)") (InputAction :type "InputAction Object Reference" :default "/Game/Input/IA_Thrust.IA_Thrust"))
  ;[0.03 0.03 0.03] Input
  (:`Triggered`
    (set `self.thrustInput` ActionValue :!label _label_2))
  (:`Completed`
    (goto _label_2)))

(event `EnhancedInput|/Game/Input/IA_Boost`
  (params (ActionValue :type Boolean) (ElapsedSeconds :type "Float (double-precision)") (TriggeredSeconds :type "Float (double-precision)") (InputAction :type "InputAction Object Reference" :default "/Game/Input/IA_Boost.IA_Boost"))
  ;[0.03 0.03 0.03] Input
  (:`Triggered`
    (set `self.boostInput` ActionValue :!label _label_3))
  (:`Completed`
    (goto _label_3)))

(event `EnhancedInput|/Game/Input/IA_Shoot`
  (params (ActionValue :type Boolean) (ElapsedSeconds :type "Float (double-precision)") (TriggeredSeconds :type "Float (double-precision)") (InputAction :type "InputAction Object Reference" :default "/Game/Input/IA_Shoot.IA_Shoot"))
  ;[0.03 0.03 0.03] Input
  (:`Triggered`
    (set `self.shootInput` ActionValue)
    (`self.OnStartedShooting`))
  (:`Completed`
    (set `self.shootInput` ActionValue)
    (`self.OnStoppedShooting`)))

(event `EnhancedInput|/Game/Input/IA_Exit`
  (params (ActionValue :type "Float (double-precision)") (ElapsedSeconds :type "Float (double-precision)") (TriggeredSeconds :type "Float (double-precision)") (InputAction :type "InputAction Object Reference" :default "/Game/Input/IA_Exit.IA_Exit"))
  ;[0.03 0.03 0.03] Input
  (:`Triggered`
    (`KismetSystemLibrary.QuitGame` null "Quit")))

(event `self.ReceiveHit`
  (params (MyComp :type "PrimitiveComponent Object Reference") (Other :type "Actor Object Reference") (OtherComp :type "PrimitiveComponent Object Reference") (bSelfMoved :type Boolean) (HitLocation :type "Vector Structure") (HitNormal :type "Vector Structure") (NormalImpulse :type "Vector Structure") (Hit :type "HitResult Structure (by ref)"))
  ;[0.03 0.03 0.03] Collisions
  (if (> (`KismetMathLibrary.VSize` NormalImpulse) (`self.MinCollisionForceForEvents`))
    (if (> (`KismetSystemLibrary.GetGameTimeInSeconds`) (+ (`self.timeLastCollided`) (`self.MinDurationBetweenCollisionEvents`)))
      (`self.OnSpaceShipCollided` (`KismetMathLibrary.VSize` NormalImpulse))
      (set `self.timeLastCollided` (`KismetSystemLibrary.GetGameTimeInSeconds`))
      (set `self.Hit Location` HitLocation))))

(event `OnThrustStateChanged`
  (params (isThrustActive :type Boolean))
  (bind _music (`self.Music`))
  ;[0.03 0.03 0.03] Movement Events
  (bind _output_get (set `self.Is Thrust Active` isThrustActive))
  (if _output_get
    (if (`self.GetIsBoosting`)
      (`self.ThrustEvents` "Thrust" 2.0)
      (else
        (`self.ThrustEvents` "Thrust" 1.0)
        (`FMODBlueprintStatics.EventInstanceSetParameter` (`self.Music`) "Game" 1.0)))
    (else
      (`self.ThrustEvents` "Thrust")
      (if (> (stale `OnForwardSpeedChanged` _output_get) 0.0)
        (`FMODBlueprintStatics.EventInstanceSetParameter` _music "Game" 3.0)
        (else
          (`FMODBlueprintStatics.EventInstanceSetParameter` _music "Game" 0.0))))))

(event `OnForwardSpeedChanged`
  (params (forwardSpeed :type "Float (double-precision)"))
  (bind _returnvalue (`KismetMathLibrary.MapRangeClamped` forwardSpeed 0.0 25000.0 0.0 10.0))
  ;[0.03 0.03 0.03] Movement Events
  (`self.ThrustEvents` "Speed" _returnvalue)
  (bind _output_get (set `self.Speed` _returnvalue)))

(event `OnSteerInputChanged`
  (params (steerInputX :type "Float (double-precision)") (steerInputY :type "Float (double-precision)"))
  (bind _steering (`self.Steering`))
  ;[0.03 0.03 0.03] Movement Events
  (`FMODBlueprintStatics.EventInstanceSetParameter` _steering "XCoord" steerInputX)
  (`FMODBlueprintStatics.EventInstanceSetParameter` _steering "YCoord" steerInputY))

(event `OnStartedBoosting`
  ;[0.03 0.03 0.03] Boosting Events
  (bind _returnvalue (`FMODBlueprintStatics.PlayEventAttached` "/Game/FMOD/Events/Spaceship/Boosting.Boosting" (`self.Spaceship`) "None" (0.0 0.0 0.0) "KeepRelativeOffset"))
  (`FMODAudioComponent.SetParameter` _returnvalue "Boosting" 1.0)
  (`FMODBlueprintStatics.EventInstanceSetParameter` (`self.Music`) "Game" 2.0))

(event `OnStoppedBoosting`
  (bind _music (`self.Music`))
  ;[0.03 0.03 0.03] Boosting Events
  (bind _returnvalue (`FMODBlueprintStatics.PlayEventAttached` "/Game/FMOD/Events/Spaceship/Boosting.Boosting" (`self.Spaceship`) "None" (0.0 0.0 0.0) "KeepRelativeOffset"))
  (`FMODAudioComponent.SetParameter` _returnvalue "Boosting" 0.0)
  (if (`self.Is Thrust Active`)
    (`FMODBlueprintStatics.EventInstanceSetParameter` _music "Game" 1.0)
    (else
      (`FMODBlueprintStatics.EventInstanceSetParameter` _music "Game" 3.0))))

(event `OnSpaceShipCollided`
  (params (collisionForce :type "Float (double-precision)"))
  ;[0.03 0.03 0.03] Collision Events
  (bind _returnvalue (`FMODBlueprintStatics.PlayEventAtLocation` "/Game/FMOD/Events/Spaceship/Collide.Collide" (`KismetMathLibrary.Conv_VectorToTransform` (`self.Hit Location`))))
  (`FMODBlueprintStatics.EventInstanceSetParameter` _returnvalue "Force" (`KismetMathLibrary.MapRangeClamped` collisionForce 0.0 30000.0 0.0 100.0)))

(event `OnShootLasers`
  ;[0.03 0.03 0.03] Shooting Lasers
  (`FMODBlueprintStatics.PlayEventAttached` "/Game/FMOD/Events/Spaceship/Shoot.Shoot" (`self.BPSC_LaserProjectile_Left`) "None" (0.0 0.0 0.0) "KeepRelativeOffset")
  (`FMODBlueprintStatics.PlayEventAttached` "/Game/FMOD/Events/Spaceship/Shoot.Shoot" (`self.BPSC_LaserProjectile_Right`) "None" (0.0 0.0 0.0) "KeepRelativeOffset"))

(event `OnStartedShooting`
  ;[0.03 0.03 0.03] Shooting Lasers
)

(event `OnStoppedShooting`
  ;[0.03 0.03 0.03] Shooting Lasers
)

(fn `AsteroidCount`
  (bind _counter (`self.Counter`))
  (if (== _counter 0)
    (`FMODBlueprintStatics.EventInstanceStop` (`self.Music`))
    (`self.EndGame`)
    (elif (== _counter 5)
      (`/Engine/EditorBlueprintResources/StandardMacros.DoOnce` false)
      (elif (== _counter 2)
        (`/Engine/EditorBlueprintResources/StandardMacros.DoOnce` false)))))

(fn `AsteroidSub`
  (bind _output_get (set `self.Counter` (- (`self.Counter`) 1)))
  (`TextBlock.SetText` (`/Game/HUD_Widget.NumAsteroids` (`self.HUD_Widget`)) (`KismetTextLibrary.Conv_IntToText` _output_get))
  (bind _returnvalue (`FMODBlueprintStatics.PlayEvent2D` "/Game/FMOD/Events/UI/PointFeedback.PointFeedback"))
  (`FMODBlueprintStatics.EventInstanceSetParameter` _returnvalue "Counter" (`KismetMathLibrary.Conv_IntToDouble` _output_get)))

(fn `EndGame`
  (`FMODBlueprintStatics.PlayEvent2D` "/Game/FMOD/Events/UI/VictorySound.VictorySound")
  (`FMODBlueprintStatics.PlayEvent2D` "/Game/FMOD/Events/Music/Victory.Victory")
  (bind _returnvalue (`|CreateWidget` "/Game/End_HUD_Widget.End_HUD_Widget_C"))
  (bind _output_get (set `self.End_Widget` _returnvalue))
  (`UserWidget.AddToViewport` _output_get 0)
  (`Widget.RemoveFromParent` (`self.HUD_Widget`))
  (set `self.boostInput` true)
  (set `self.shootInput` false)
  (`Controller.UnPossess` (`GameplayStatics.GetPlayerController` 0))
  (`FMODBlueprintStatics.EventInstanceStop` (`self.Ambience`)))

(fn `ThrustEvents`
  (params (Param :type Name) (Value :type "Float (double-precision)"))
  (`FMODAudioComponent.SetParameter` (`self.ThrustEvent_L`) Param Value)
  (`FMODAudioComponent.SetParameter` (`self.ThrustEvent_R`) Param Value))

(fn `UserConstructionScript`)